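; Anim notify state that drives ranged attack hit detection during an animation window, part of the Parry Attack System.
; Each tick it finds the AC_Hitbox component on the mesh owner and sends a begin ranged trace message with the notify's height, radius and forward length.
; When the window ends it tells the same component to end the attack trace.
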(fn GetNotifyName
  (return "Hitbox Ranged Notify"))

(fn ReceivedNotifyEnd
  (params (MeshComp :type Skeletal%20Mesh%20Component%20Object%20Reference) (Animation :type Anim%20Sequence%20Base%20Object%20Reference) (EventReference :type Anim%20Notify%20Event%20Reference%20Structure%20%28by%20ref%29))
  (Class|BIHitbox|EndAttackTrace(Message) (Actor|GetComponentbyClass (Components|GetOwner MeshComp) "/Game/ParryAttackSystem/PAS_Assets/HitboxComponent/BluePrint/AC_Hitbox.AC_Hitbox_C"))
  (return false))

(fn ReceivedNotifyTick
  (params (MeshComp :type Skeletal%20Mesh%20Component%20Object%20Reference) (Animation :type Anim%20Sequence%20Base%20Object%20Reference) (FrameDeltaTime :type Float%20%28single-precision%29) (EventReference :type Anim%20Notify%20Event%20Reference%20Structure%20%28by%20ref%29))
  (Class|BIHitbox|BeginRangedAttackTrace(Message) (Actor|GetComponentbyClass (Components|GetOwner MeshComp) "/Game/ParryAttackSystem/PAS_Assets/HitboxComponent/BluePrint/AC_Hitbox.AC_Hitbox_C") (Variables|Default|GetTraceHeight) (Variables|Default|GetTrace%20Radius) (Variables|Default|GetTrace%20Forward%20Length))
  (return false))