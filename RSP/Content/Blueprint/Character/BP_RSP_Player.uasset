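; BP_RSP_Player is a player character Blueprint that spawns force fields at hit points and triggers a Gameplay Ability.
; CreateHitPoint offsets the actor's location 200 units along world X, since the forward vector uses a zero rotation rather than the actor's, and passes it to AddForce.
; AddForce spawns an FS_MasterField there.
; Pressing Q calls TryActivateAbilityByClass on the Ability System Component, with no ability class shown.
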(event Custom|AddForce
  (params (SpawnTransform :type Transform))
  (Game|SpawnActorfromClass "/Engine/EditorResources/FieldNodes/FS_MasterField.FS_MasterField_C" SpawnTransform "Undefined" "MultiplyWithRoot" 0 0))

(event EventBeginPlay)

(event Collision|EventActorBeginOverlap
  (params (OtherActor :type Actor%20Object%20Reference)))

(event EventTick
  (params (DeltaSeconds :type Float%20%28single-precision%29)))

(event EventCreateHitPoint
  (CallFunction|AddForce (Math|Conversions|ToTransform(Vector) (+ (.Location (Math|Transform|BreakTransform (Transformation|GetActorTransform))) (* (Math|Vector|GetForwardVector "0, 0, 0") "200.000000,200.000000,0.000000") ""))))

(event Input|KeyboardEvents|Q
  (params (Key :type Key%20Structure :default "None"))
  (:Pressed
    (Abilities|TryActivateAbilitybyClass (Ability|GetAbilitySystemComponent 0) 0 true)))

(fn ConstructionScript)